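; Fireplace actor that flickers its glow and consumes books that enter its trigger box.
; Tick drives two lights, each getting a new random intensity after short random delays.
; A box overlap increments TotalBooks on the BookInstance game instance, then after a brief delay destroys the overlapping Book_Blueprint.
; The count rises before the book cast, so any overlapping actor adds to it.
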(event OnComponentBeginOverlap(Box)
  (params (OverlappedComponent :type Primitive%20Component%20Object%20Reference) (OtherActor :type Actor%20Object%20Reference) (OtherComp :type Primitive%20Component%20Object%20Reference) (OtherBodyIndex :type Integer) (bFromSweep :type Boolean) (SweepResult :type Hit%20Result%20Structure%20%28by%20ref%29))
  (bind _asbook_instance (Utilities|Casting|CastToBookInstance (Game|GetGameInstance)))
  (Variables|/Game/FirstPersonBP/Blueprints/BookInstance.BookInstance_C|SettotalBooks _asbook_instance (+ (Variables|/Game/FirstPersonBP/Blueprints/BookInstance.BookInstance_C|GettotalBooks _asbook_instance) 1))
  (Utilities|FlowControl|Delay 0.4)
  (bind _asbook_blueprint (Utilities|Casting|CastToBook_Blueprint OtherActor))
  (Actor|DestroyActor _asbook_blueprint))

(event EventBeginPlay)

(event Collision|EventActorBeginOverlap
  (params (OtherActor :type Actor%20Object%20Reference)))

(event EventTick
  (params (DeltaSeconds :type Float%20%28single-precision%29))
  (Utilities|FlowControl|Sequence
    (:then_0
      (Utilities|FlowControl|Delay (Math|Random|RandomFloatinRange 0.0 0.2))
      (Rendering|Components|Light|SetIntensity (Variables|Default|Getfireglow2) (Class|KismetMathLibrary|FInterpEaseinOut (Math|Random|RandomFloatinRange 2.5e+03 1e+04) (Math|Random|RandomFloatinRange 2.5e+03 1e+04) 1.0 1.0)))
    (:then_1
      (Utilities|FlowControl|Delay (Math|Random|RandomFloatinRange 0.0 0.2))
      (Rendering|Components|Light|SetIntensity (Variables|Default|GetfireGlow) (Class|KismetMathLibrary|FInterpEaseinOut (Math|Random|RandomFloatinRange 2.5e+03 1e+04) (Math|Random|RandomFloatinRange 2.5e+03 1e+04) 0.5 1.0)))))

(fn ConstructionScript)